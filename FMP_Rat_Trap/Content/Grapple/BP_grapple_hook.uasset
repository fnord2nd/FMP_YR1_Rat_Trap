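; Grapple hook projectile actor that flies in a straight line to a Target actor and stops there.
; On BeginPlay it caches start and end locations and launches its ProjectileMovement along that direction at SpeedOfGrappleHook.
; Tick compares squared distances from the start against the Target's live location, then snaps to the cached endpoint and zeroes velocity.
; DistanceToTarget returns the remaining distance to that endpoint.
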(event `self.ReceiveBeginPlay`
  (set `self.starting location` (`self.K2_GetActorLocation`))
  (set `self.ending location` (`self.K2_GetActorLocation` (`self.target`)))
  (set `self.dierection` (`KismetMathLibrary.Normal` (- (`self.ending location`) (`self.starting location`))))
  (set `MovementComponent.Velocity` (* (`self.dierection`) (`self.speed of grapple hook`)) (`self.ProjectileMovement`)))

(event `self.ReceiveTick`
  (params (DeltaSeconds :type "Float (single-precision)"))
  (if (>= (`KismetMathLibrary.Vector_DistanceSquared` (`self.K2_GetActorLocation`) (`self.starting location`)) (`KismetMathLibrary.Vector_DistanceSquared` (`self.K2_GetActorLocation` (`self.target`)) (`self.starting location`)))
    (`self.K2_SetActorLocation` (+ (`self.starting location`) (* (`self.dierection`) (`KismetMathLibrary.Vector_Distance` (`self.starting location`) (`self.ending location`)))) false true)
    (set `MovementComponent.Velocity` (0.0 0.0 0.0) (`self.ProjectileMovement`))))

(fn `distance to target`
  (returns (ReturnValue :type "Float (double-precision)"))
  (return (`KismetMathLibrary.Vector_Distance` (`self.ending location`) (`self.K2_GetActorLocation`))))

(fn `UserConstructionScript`)