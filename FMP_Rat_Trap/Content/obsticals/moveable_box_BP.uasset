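; Movable box obstacle that the player can push only while standing in one of its trigger volumes.
; Two collision components, one for the X axis and one for the Y axis, enable physics simulation on the Cube when a ThirdPersonCharacter begins overlapping.
; Either volume disables simulation when the character leaves it, with no check on whether the other is still overlapped.
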(event `self.y ax collision.OnComponentBeginOverlap`
  (params (OverlappedComponent :type "PrimitiveComponent Object Reference") (OtherActor :type "Actor Object Reference") (OtherComp :type "PrimitiveComponent Object Reference") (OtherBodyIndex :type Integer) (bFromSweep :type Boolean) (SweepResult :type "HitResult Structure (by ref)"))
  (cast `/Game/ThirdPersonBP/Blueprints/ThirdPersonCharacter` OtherActor)
  (`PrimitiveComponent.SetSimulatePhysics` (`self.cube`) true))

(event `self.y ax collision.OnComponentEndOverlap`
  (params (OverlappedComponent :type "PrimitiveComponent Object Reference") (OtherActor :type "Actor Object Reference") (OtherComp :type "PrimitiveComponent Object Reference") (OtherBodyIndex :type Integer))
  (cast `/Game/ThirdPersonBP/Blueprints/ThirdPersonCharacter` OtherActor)
  (`PrimitiveComponent.SetSimulatePhysics` (`self.cube`) false))

(event `self.x ax collision.OnComponentBeginOverlap`
  (params (OverlappedComponent :type "PrimitiveComponent Object Reference") (OtherActor :type "Actor Object Reference") (OtherComp :type "PrimitiveComponent Object Reference") (OtherBodyIndex :type Integer) (bFromSweep :type Boolean) (SweepResult :type "HitResult Structure (by ref)"))
  (cast `/Game/ThirdPersonBP/Blueprints/ThirdPersonCharacter` OtherActor)
  (`PrimitiveComponent.SetSimulatePhysics` (`self.cube`) true))

(event `self.x ax collision.OnComponentEndOverlap`
  (params (OverlappedComponent :type "PrimitiveComponent Object Reference") (OtherActor :type "Actor Object Reference") (OtherComp :type "PrimitiveComponent Object Reference") (OtherBodyIndex :type Integer))
  (cast `/Game/ThirdPersonBP/Blueprints/ThirdPersonCharacter` OtherActor)
  (`PrimitiveComponent.SetSimulatePhysics` (`self.cube`) false))

(fn `UserConstructionScript`)